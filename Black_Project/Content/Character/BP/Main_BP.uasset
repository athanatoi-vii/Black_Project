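; Player character Blueprint for a pistol that grabs, carries and manipulates physics objects, gravity-gun style.
; While standing, a per-tick laser-socket trace selects a simulating component; attack start attaches it to the pistol with heavy linear damping.
; Input events push, pull and rotate the held object.
; It detaches when attack or standing ends, the trace loses it, or a box trace finds contact above speed thresholds computed from frame-to-frame movement.
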(event Custom|Collision
  (bind _oj (Variables|Default|GetOJ))
  (bind _returnvalue (Transformation|GetWorldLocation _oj))
  (if (not (Variables|Default|GetbOJ))
    (bind (_outhit _returnvalue_2) (Collision|BoxTraceByChannel _returnvalue _returnvalue (+ (Transformation|GetWorldScale _oj) 60) (Transformation|GetWorldRotation _oj) "TraceTypeQuery1" false (Utilities|Array|MakeArray (Components|GetOwner _oj)) "ForOneFrame" false "(R=1.000000,G=0.470967,B=0.000000,A=1.000000)" "(R=1.000000,G=0.470967,B=0.000000,A=1.000000)" (Utilities|Time|GetWorldDeltaSeconds)))
    (bind _speed (CallFunction|BalckVelocity (Variables|Default|GetOJ)))
    (if _returnvalue_2
      (if (Physics|IsSimulatingPhysics (.HitComponent (Collision|BreakHitResult _outhit)) "None")
        (if (> _speed 4e+03)
          (CallFunction|DettachCollision :!label _label))
        (elif (> _speed 2.5e+03)
          (goto _label))))))

(event Custom|Set%20OJ
  (bind _pistol (Variables|Default|GetPistol))
  (bind _returnvalue (Transformation|GetSocketLocation _pistol "Liser"))
  (if (Variables|Default|GetbStanding)
    (bind (_outhit _returnvalue_2) (Collision|LineTraceByChannel _returnvalue (+ _returnvalue (* (Math|Vector|GetForwardVector (Transformation|GetSocketRotation _pistol "Liser")) 9e+02)) "TraceTypeQuery1" false 0 "ForOneFrame" true "(R=1.000000,G=0.470967,B=0.000000,A=1.000000)" "(R=1.000000,G=1.000000,B=1.000000,A=0.000000)" (Utilities|Time|GetWorldDeltaSeconds)))
    (if (Variables|Default|GetbOJ)
      (if _returnvalue_2
        (if (Physics|IsSimulatingPhysics (.HitComponent (Collision|BreakHitResult _outhit)) "None")
          (if (Utilities|Enum|NotEqual(Enum) (Utilities|GetDisplayName (.HitComponent (Collision|BreakHitResult _outhit))) (Utilities|GetDisplayName (Variables|Default|GetOJ)))
            (Variables|Default|SetOJ (.HitComponent (Collision|BreakHitResult _outhit))))
          (else
            (Utilities|IsValid (Variables|Default|GetOJ)
              (:Is%20Valid
                (Variables|Default|SetOJ 0)))))
        (else
          (Utilities|IsValid (Variables|Default|GetOJ)
            (:Is%20Valid
              (Variables|Default|SetOJ 0)))))
      (elif _returnvalue_2
        (if (Utilities|Enum|NotEqual(Enum) (Utilities|GetDisplayName (.HitComponent (Collision|BreakHitResult _outhit))) (Utilities|GetDisplayName (Variables|Default|GetOJ)))
          (CallFunction|DettachCollision :!label _label))
        (else
          (goto _label))))))

(event Custom|Dettach_Collision
  (bind _oj (Variables|Default|GetOJ))
  (if (not (Variables|Default|GetbOJ))
    (Physics|SetSimulatePhysics _oj true)
    (Class|PrimitiveComponent|SetLinearDamping _oj 0.1)
    (Transformation|DetachFromComponent (Variables|Default|GetOJ) "KeepWorld" "KeepWorld" "KeepWorld" true)
    (Variables|Default|SetbOJ true)))

(event EventRotateRBP
  (params (Value :type Input%20Action%20Value%20Structure%20%28by%20ref%29))
  (if (not (Variables|Default|GetbOJ))
    (Transformation|AddLocalRotation (Variables|Default|GetOJ) (Math|Rotator|MakeRotator (* (Input|EnhancedActionValues|GetIA_Rotate_R) (Variables|Default|GetfRotate_Reverse)) 0.0 0.0) false false)))

(event EventTick
  (params (DeltaSeconds :type Float%20%28single-precision%29))
  (CallFunction|SetOJ)
  (CallFunction|Collision))

(event EventRotatePBP
  (params (Value :type Input%20Action%20Value%20Structure%20%28by%20ref%29))
  (if (not (Variables|Default|GetbOJ))
    (Transformation|AddLocalRotation (Variables|Default|GetOJ) (Math|Rotator|MakeRotator 0.0 (* (Input|EnhancedActionValues|GetIA_Rotate_P) (Variables|Default|GetfRotate_Reverse)) 0.0) false false)))

(event EventFuncAttackEndBP
  (bind _oj (Variables|Default|GetOJ))
  (if (not (Variables|Default|GetbOJ))
    (Physics|SetSimulatePhysics _oj true)
    (Class|PrimitiveComponent|SetLinearDamping _oj 0.1)
    (Transformation|DetachFromComponent (Variables|Default|GetOJ) "KeepWorld" "KeepWorld" "KeepWorld" true)
    (Variables|Default|SetbOJ true)))

(event EventFuncAttackStartBP
  (bind _oj (Variables|Default|GetOJ))
  (Utilities|IsValid _oj
    (:Is%20Valid
      (Physics|SetSimulatePhysics _oj true)
      (Class|PrimitiveComponent|SetLinearDamping _oj 1e+03)
      (bind _returnvalue (Transformation|AttachComponentToComponent _oj (Variables|Default|GetPistol) "OJ" "KeepWorld" "KeepWorld" "KeepWorld" true))
      (if _returnvalue
        (Variables|Default|SetOJ_Location (Transformation|GetActorLocation (Components|GetOwner (Variables|Default|GetOJ))))
        (Variables|Default|SetbOJ false)))))

(event EventRotateYBP
  (params (Value :type Input%20Action%20Value%20Structure%20%28by%20ref%29))
  (bind _returnvalue (Input|EnhancedActionValues|GetIA_Rotate_Y))
  (if (not (Variables|Default|GetbOJ))
    (Transformation|AddLocalRotation (Variables|Default|GetOJ) (Math|Rotator|MakeRotator (* _returnvalue (Variables|Default|GetfRotate_Reverse)) 0.0 _returnvalue) false false)))

(event EventFuncStandingEndBP
  (params (Value :type Input%20Action%20Value%20Structure%20%28by%20ref%29))
  (bind _oj (Variables|Default|GetOJ))
  (if (not (Variables|Default|GetbOJ))
    (Physics|SetSimulatePhysics _oj true)
    (Class|PrimitiveComponent|SetLinearDamping _oj 0.1)
    (Transformation|DetachFromComponent (Variables|Default|GetOJ) "KeepWorld" "KeepWorld" "KeepWorld" true)
    (Variables|Default|SetbOJ true)))

(event EventFuncSpaceBP
  (params (Value :type Input%20Action%20Value%20Structure%20%28by%20ref%29))
  (bind _returnvalue (Input|EnhancedActionValues|GetIA_Space))
  (bind _frotate_reverse (Variables|Default|GetfRotate_Reverse))
  (bind _oj (Variables|Default|GetOJ))
  (bind _pistol (Variables|Default|GetPistol))
  (bind _returnvalue_2 (Transformation|GetWorldLocation _oj))
  (bind _returnvalue_3 (Transformation|GetWorldLocation _pistol))
  (bind _returnvalue_4 (* _returnvalue _frotate_reverse))
  (bind _returnvalue_5 (Math|Vector|Distance(Vector) _returnvalue_2 _returnvalue_3))
  (if (not (Variables|Default|GetbOJ))
    (if (or (and (< _returnvalue_4 0.0) (> _returnvalue_5 1.2e+02)) (and (> _returnvalue_4 0.0) (< _returnvalue_5 895.0)))
      (Transformation|SetWorldLocation _oj (+ (Transformation|GetWorldLocation _oj) (* (Math|Vector|GetForwardVector (Transformation|GetWorldRotation _pistol)) (* _returnvalue_4 15.0))) false false))))

(fn ConstructionScript)

(fn BalckVelocity
  (params (OJ :type Primitive%20Component%20Object%20Reference))
  (bind _returnvalue (Components|GetOwner OJ))
  (bind _returnvalue_2 (Transformation|GetActorLocation _returnvalue))
  (Variables|Default|SetOJ_Speed (Math|Vector|VectorLength (/ (- _returnvalue_2 (Variables|Default|GetOJ_Location)) (Utilities|Time|GetWorldDeltaSeconds))))
  (Variables|Default|SetOJ_Location _returnvalue_2)
  (return (Variables|Default|GetOJ_Speed)))